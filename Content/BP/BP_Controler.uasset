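; BP_Controler runs the in-game work shift clock and creates the related UI.
; On BeginPlay it adds the HUD widget and starts a looping timer at the TimeSpeed interval.
; Each tick of that timer advances Minute and rolls it over into Hour.
; When Hour reaches 18, it sets ShiftEnded, clears the timer and shows the shift-ended widget.
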(event Custom|IncreaseTime
  (Variables|Default|SetMinute (+ (Variables|Default|GetMinute) 1))
  (if (>= (Variables|Default|GetMinute) 60)
    (Variables|Default|SetMinute 0)
    (Variables|Default|SetHour (+ (Variables|Default|GetHour) 1))
    (if (== (Variables|Default|GetHour) 18)
      (Variables|Default|SetShiftEnded true)
      (Utilities|Time|ClearandInvalidateTimerbyHandle (stale EventBeginPlay _returnvalue))
      (bind _returnvalue (UserInterface|CreateWidget "/Game/BP/UI/WBP_ShiftEnded.WBP_ShiftEnded_C"))
      (UserInterface|Viewport|AddtoViewport _returnvalue 0))))

(event EventBeginPlay
  (bind _returnvalue (Utilities|Time|SetTimerbyEvent (delegate Custom|IncreaseTime) (Variables|Default|GetTimeSpeed) true))
  (bind _returnvalue_2 (UserInterface|CreateWidget "/Game/BP/UI/WBP_HUD.WBP_HUD_C" (Game|GetPlayerController 0)))
  (UserInterface|Viewport|AddtoViewport _returnvalue_2 0))

(fn ConstructionScript)