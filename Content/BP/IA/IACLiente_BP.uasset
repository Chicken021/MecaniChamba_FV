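; Customer AI pawn that walks to a TargetPoint on BeginPlay, retrying on failure, and waits to be served.
; Once waiting, a timer makes it leave angry and destroy itself if ignored too long.
; Clicking its capsule while it waits and the player character is flagged near it adds random money to BP_Controler's TotalMoney and destroys the customer.
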(event OnClicked(CapsuleComponent)
  (params (TouchedComponent :type Primitive%20Component%20Object%20Reference) (ButtonPressed :type Key%20Structure :default "None"))
  (if (and (Variables|Default|GetIsWaiting) (Variables|/Game/TopDown/Blueprints/BP_TopDownCharacter.BP_TopDownCharacter_C|GetIsNearTheClient (.AsBP%20Top%20Down%20Character (Utilities|Casting|CastToBP_TopDownCharacter (Game|GetPlayerCharacter 0)))))
    (Development|PrintString "Atiendeme ")
    (bind _returnvalue (Actor|GetActorOfClass "/Game/BP/BP_Controler.BP_Controler_C"))
    (bind _output_get (Variables|Default|SetMoney (Math|Random|RandomIntegerinRange 300 700)))
    (Variables|/Game/BP/BP_Controler.BP_Controler_C|SetTotalMoney _returnvalue (+ (Variables|/Game/BP/BP_Controler.BP_Controler_C|GetTotalMoney _returnvalue) _output_get))
    (Development|PrintString "Gracias")
    (Actor|DestroyActor)))

(event Custom|Cliente%20enojado
  (Development|PrintString "Bye")
  (Actor|DestroyActor))

(event EventBeginPlay
  (bind _returnvalue (Actor|GetActorOfClass "/Script/Engine.TargetPoint" :!label _label))
  (AI|AIMoveTo self "0, 0, 0" _returnvalue 5.0 false
    (:OnSuccess
      (Development|PrintString "esperando a que me atiendan ")
      (Variables|Default|SetIsWaiting true)
      (Utilities|Time|SetTimerbyEvent (delegate Custom|Cliente%20enojado) 4e+01))
    (:OnFail
      (Utilities|FlowControl|Delay 2.0)
      (goto _label))))

(event Collision|EventActorBeginOverlap
  (params (OtherActor :type Actor%20Object%20Reference)))

(event EventTick
  (params (DeltaSeconds :type Float%20%28single-precision%29)))

(fn ConstructionScript)