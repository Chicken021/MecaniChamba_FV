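; BP_NewBasicMachine is a money-producing machine that pays out on a looping timer and can randomly break, swapping to a broken material.
; Payouts go to BP_Controler's total if auto-collect is on or the player is inside the collection box; otherwise they accumulate until the player enters.
; A widget component shows stored money and the countdown.
; A second trigger opens the WBP_RepairMachine widget while broken and removes it on exit.
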(event OnComponentBeginOverlap(Box)
  (params (OverlappedComponent :type Primitive%20Component%20Object%20Reference) (OtherActor :type Actor%20Object%20Reference) (OtherComp :type Primitive%20Component%20Object%20Reference) (OtherBodyIndex :type Integer) (bFromSweep :type Boolean) (SweepResult :type Hit%20Result%20Structure%20%28by%20ref%29))
  ;[0.15 0.15 0.15 0.5] Se realiza el cobro al pasar por la zona y se actualiza el dinero
  (Utilities|Casting|CastToBP_TopDownCharacter OtherActor)
  (Variables|Default|SetPlayerInZone true)
  (if (> (Variables|Default|GetDineroAcumulado) 0)
    (bind _returnvalue (Actor|GetActorOfClass "/Game/BP/BP_Controler.BP_Controler_C"))
    (Variables|/Game/BP/BP_Controler.BP_Controler_C|SetDineroTotal _returnvalue (+ (Variables|/Game/BP/BP_Controler.BP_Controler_C|GetDineroTotal _returnvalue) (Variables|Default|GetDineroAcumulado)))
    (bind _output_get (Variables|Default|SetDineroAcumulado 0))
    (Rendering|Components|TextRender|SetText (Variables|/Game/BP/UI/WBP_MachineHUD.WBP_MachineHUD_C|GetMonettxt (Variables|Default|GetHUDInstance)) (Utilities|Text|FormatText "Money: ${cant}" _output_get))))

(event OnComponentEndOverlap(Box)
  (params (OverlappedComponent :type Primitive%20Component%20Object%20Reference) (OtherActor :type Actor%20Object%20Reference) (OtherComp :type Primitive%20Component%20Object%20Reference) (OtherBodyIndex :type Integer))
  ;[0.15 0.15 0.15 0.5] Si el jugador no esta en la zona se vuelve falso
  (Utilities|Casting|CastToBP_TopDownCharacter OtherActor)
  (Variables|Default|SetPlayerInZone false))

(event OnComponentBeginOverlap(DeteccionReparacion)
  (params (OverlappedComponent :type Primitive%20Component%20Object%20Reference) (OtherActor :type Actor%20Object%20Reference) (OtherComp :type Primitive%20Component%20Object%20Reference) (OtherBodyIndex :type Integer) (bFromSweep :type Boolean) (SweepResult :type Hit%20Result%20Structure%20%28by%20ref%29))
  ;[0.15 0.15 0.15 0.5] Si el jugador entra en la zona y la maquina esat rota salle el menu
  (Utilities|Casting|CastToBP_TopDownCharacter OtherActor)
  (if (Variables|Default|GetEstaRota)
    (bind _returnvalue (UserInterface|CreateWidget "/Game/BP/UI/WBP_RepairMachine.WBP_RepairMachine_C" 0 self))
    (bind _output_get (Variables|Default|SetReferenceToHUd _returnvalue))
    (UserInterface|Viewport|AddtoViewport _output_get 0)))

(event OnComponentEndOverlap(DeteccionReparacion)
  (params (OverlappedComponent :type Primitive%20Component%20Object%20Reference) (OtherActor :type Actor%20Object%20Reference) (OtherComp :type Primitive%20Component%20Object%20Reference) (OtherBodyIndex :type Integer))
  (bind _referencetohud (Variables|Default|GetReferenceToHUd))
  ;[0.15 0.15 0.15 0.5] Si el jugador sale de la zona rota desaparace el HUd
  (Utilities|Casting|CastToBP_TopDownCharacter OtherActor)
  (Utilities|IsValid _referencetohud
    (:Is%20Valid
      (Widget|RemovefromParent _referencetohud))))

(event Custom|ProducirDinero
  ;[0.15 0.15 0.15 0.5] Filtro para saber si esta rota y asignar la probalidad
  (if (not (Variables|Default|GetEstaRota))
    (if (<= (Math|Random|RandomFloatinRange 0.0 1.0) (Variables|Default|GetProabilidadRotura))
      ;[0.15 0.15 0.15 0.5] Esta rota cambia el color
      (Variables|Default|SetEstaRota true)
      (Rendering|Material|SetMaterial (Variables|Default|GetCube) 0 "/Game/Materials/Broken_Machine.Broken_Machine")
      (elif (Variables|Default|GetAutocollect)
        ;[0.15 0.15 0.15 0.5 10] Si Autocollect es verdadero
        (bind _returnvalue (Actor|GetActorOfClass "/Game/BP/BP_Controler.BP_Controler_C" :!label _label))
        (Variables|/Game/BP/BP_Controler.BP_Controler_C|SetDineroTotal _returnvalue (+ (Variables|/Game/BP/BP_Controler.BP_Controler_C|GetDineroTotal _returnvalue) (Variables|Default|GetCantidadDinero)))
        (else
          ;[0.15 0.15 0.15 0.5 10] Si autocollect es false aun asi se detectaque el jugador esta en zona y se suma el dinero dirrectamente
          (if (Variables|Default|GetPlayerInZone)
            (goto _label)
            (else
              ;[0.15 0.15 0.15 0.5 10] El jugador no esta en zona por lo que la maquina guarda su propio dinero
              (bind _output_get (Variables|Default|SetDineroAcumulado (+ (Variables|Default|GetDineroAcumulado) (Variables|Default|GetCantidadDinero))))
              (Rendering|Components|TextRender|SetText (Variables|/Game/BP/UI/WBP_MachineHUD.WBP_MachineHUD_C|GetMonettxt (Variables|Default|GetHUDInstance)) (Utilities|Text|FormatText "Money: ${cant}" _output_get)))))))))

(event EventTick
  (params (DeltaSeconds :type Float%20%28single-precision%29))
  ;[0.15 0.15 0.15 0.5] ActulizarHudTimer
  (if (not (Variables|Default|GetEstaRota))
    (Rendering|Components|TextRender|SetText (Variables|/Game/BP/UI/WBP_MachineHUD.WBP_MachineHUD_C|GetTimetxt (Variables|Default|GetHUDInstance)) (Utilities|Text|FormatText "{cant}s" (Utilities|Time|GetTimerRemainingTimebyHandle (Variables|Default|GetTimreHandle))))))

(event EventBeginPlay
  ;[0.15 0.15 0.15 0.5] Guarda material original
  (Variables|Default|SetMaterialOriginal (Rendering|Material|GetMaterial (Variables|Default|GetCube) 0))
  ;[0.15 0.15 0.15 0.5] Timer para Generar Dinero
  (bind _returnvalue (Utilities|Time|SetTimerbyEvent (delegate Custom|ProducirDinero) (Variables|Default|GetTiempProduccion) true))
  (Variables|Default|SetTimreHandle _returnvalue)
  ;[0.15 0.15 0.15 0.5] Instanciar MachineHUD
  (bind _aswbp_machine_hud (Utilities|Casting|CastToWBP_MachineHUD (UserInterface|GetUserWidgetObject (Variables|Default|GetMachineHUD))))
  (bind _output_get (Variables|Default|SetHUDInstance _aswbp_machine_hud))
  (Rendering|Components|TextRender|SetText (Variables|/Game/BP/UI/WBP_MachineHUD.WBP_MachineHUD_C|GetMonettxt _output_get) (Utilities|Text|FormatText "Money: ${cant}" (Variables|Default|GetDineroAcumulado))))

(fn ConstructionScript)