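; BP_Machine is a money-producing machine that accumulates income for the player to collect.
; A randomly delayed one-second timer drives a production countdown, paying BP_Controler's TotalMoney directly while BP_TopDownCharacter stands in CollecterZone, otherwise storing it.
; Entering the zone transfers stored money to the controller.
; Each completed cycle has an 80% chance to break the machine, swapping its material and halting production, with no repair logic here.
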(event OnComponentBeginOverlap(CollecterZone)
  (params (OverlappedComponent :type Primitive%20Component%20Object%20Reference) (OtherActor :type Actor%20Object%20Reference) (OtherComp :type Primitive%20Component%20Object%20Reference) (OtherBodyIndex :type Integer) (bFromSweep :type Boolean) (SweepResult :type Hit%20Result%20Structure%20%28by%20ref%29))
  (Utilities|Casting|CastToBP_TopDownCharacter OtherActor)
  (Variables|Default|SetPlayerInside true)
  (CallFunction|CollectMoney))

(event OnComponentEndOverlap(CollecterZone)
  (params (OverlappedComponent :type Primitive%20Component%20Object%20Reference) (OtherActor :type Actor%20Object%20Reference) (OtherComp :type Primitive%20Component%20Object%20Reference) (OtherBodyIndex :type Integer))
  (Utilities|Casting|CastToBP_TopDownCharacter OtherActor)
  (Variables|Default|SetPlayerInside false))

(event Custom|UpdateTimer
  (CallFunction|Production))

(event EventBeginPlay
  (Utilities|FlowControl|Delay (Math|Random|RandomFloatinRange 0.0 2.0))
  (Utilities|Time|SetTimerbyEvent (delegate Custom|UpdateTimer) 1.0 true))

(fn ConstructionScript)

(fn Production
  (if (not (Variables|Default|GetIsBroken))
    (Rendering|Material|SetMaterial (Variables|Default|GetCube) 0 "/Game/Materials/ActiveMachine.ActiveMachine")
    (Variables|Default|SetActualTime (- (Variables|Default|GetActualTime) 1.0))
    (if (<= (Variables|Default|GetActualTime) 0.0)
      (if (Variables|Default|GetPlayerInside)
        (CallFunction|CampMoney)
        (else
          (Variables|Default|SetMoneyAcumulate (+ (Variables|Default|GetMoneyAcumulate) (Variables|Default|GetMoneyProduction)))))
      (CallFunction|CheckMachineState)
      (Variables|Default|SetActualTime (Variables|Default|GetBaseTime)))))

(fn CollectMoney
  (bind _returnvalue (Actor|GetActorOfClass "/Game/BP/BP_Controler.BP_Controler_C"))
  (Variables|/Game/BP/BP_Controler.BP_Controler_C|SetTotalMoney _returnvalue (+ (Variables|Default|GetMoneyAcumulate) (Variables|/Game/BP/BP_Controler.BP_Controler_C|GetTotalMoney _returnvalue)))
  (Variables|Default|SetMoneyAcumulate 0))

(fn CampMoney
  (bind _returnvalue (Actor|GetActorOfClass "/Game/BP/BP_Controler.BP_Controler_C"))
  (Variables|/Game/BP/BP_Controler.BP_Controler_C|SetTotalMoney _returnvalue (+ (Variables|Default|GetMoneyProduction) (Variables|/Game/BP/BP_Controler.BP_Controler_C|GetTotalMoney _returnvalue))))

(fn CheckMachineState
  (if (not (< (Math|Random|RandomFloat) 0.2))
    (Variables|Default|SetIsBroken true)
    (Development|PrintString "Maquina Rota")
    (Rendering|Material|SetMaterial (Variables|Default|GetCube) 0 "/Game/Materials/Broken_Machine.Broken_Machine")))